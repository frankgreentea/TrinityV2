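; Respawn volume that sends the player back to a saved checkpoint and resets pickable cubes that touch it.
; Overlap triggers the respawn event for the player character, or CubeRespawn on a Pickable_Cube.
; Respawn loads the save, matches TestRoomProgress to the number suffix in PlayerStart names, then applies that start's location and rotation, printing the progress.
; The construction script tints the volume's glass material.
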(event OnComponentBeginOverlap(Cube)
  (params (OverlappedComponent :type Primitive%20Component%20Object%20Reference) (OtherActor :type Actor%20Object%20Reference) (OtherComp :type Primitive%20Component%20Object%20Reference) (OtherBodyIndex :type Integer) (bFromSweep :type Boolean) (SweepResult :type Hit%20Result%20Structure%20%28by%20ref%29))
  (Utilities|Casting|CastToBP_MyCharacter OtherActor
    (:then
      (CallFunction|RespawnEvent))
    (:CastFailed
      (bind _aspickable_cube (Utilities|Casting|CastToPickable_Cube OtherActor))
      (Default|CubeRespawn _aspickable_cube))))

(event Custom|Respawn_event
  ;[1 1 1] StreamLevel
  (bind _returnvalue (SaveGame|LoadGamefromSlot "SaveSlot"))
  (bind _asbp_my_save_game (Utilities|Casting|CastToBP_MySaveGame _returnvalue))
  (bind _outactors (Actor|GetAllActorsOfClass "/Script/Engine.PlayerStart"))
  (for _array_element _outactors
    (if (== (Variables|/Game/BaseGame/BP_MySaveGame.BP_MySaveGame_C|GetTestRoomProgress _asbp_my_save_game) (Math|Conversions|ToInteger(Byte) (Utilities|String|RightChop (Utilities|GetObjectName _array_element) 11)))
      (Transformation|SetActorLocation (Game|GetPlayerCharacter 0) (Transformation|GetActorLocation _array_element) false false)
      (Pawn|SetControlRotation (Game|GetPlayerController 0) (Transformation|GetActorRotation _array_element))
      (Development|PrintString (Utilities|String|ToString(Integer) (Variables|/Game/BaseGame/BP_MySaveGame.BP_MySaveGame_C|GetTestRoomProgress _asbp_my_save_game)) true true "(R=1.000000,G=0.000000,B=0.048831,A=1.000000)" 25.0))))

(event EventBeginPlay)

(event Collision|EventActorBeginOverlap
  (params (OtherActor :type Actor%20Object%20Reference)))

(event EventTick
  (params (DeltaSeconds :type Float%20%28single-precision%29)))

(fn ConstructionScript
  (Rendering|Material|SetVectorParameterValueonMaterials (Variables|Default|GetCube) "ColorGlass" (Variables|Default|GetColor)))