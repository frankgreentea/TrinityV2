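; Wall block that either blocks pawns (blue, BlocPlayer) or lets them through while blocking custom channels, apparently for shots (green, BlocTir).
; Construction script, BeginPlay and TunrOn set collision and material from BlocPlayer, IsMovable and IsDeactivable.
; Other events toggle visibility and collision or switch the type at runtime.
; Wwise provides ambience with a Blue/Green switch, and two triggers post type-specific overlap sounds on an array of Ak components.
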(event OnComponentBeginOverlap(TriggerBlue)
  (params (OverlappedComponent :type Primitive%20Component%20Object%20Reference) (OtherActor :type Actor%20Object%20Reference) (OtherComp :type Primitive%20Component%20Object%20Reference) (OtherBodyIndex :type Integer) (bFromSweep :type Boolean) (SweepResult :type Hit%20Result%20Structure%20%28by%20ref%29))
  (if (Variables|Default|GetisOn)
    (if (Variables|Default|GetBlocPlayer)
      (for _array_element (Variables|Default|GetaK_aRRAY)
        (Class|AkComponent|PostAkEvent _array_element "/Game/AudioEvents/Wall_Blue_Touch.Wall_Blue_Touch")))))

(event OnComponentBeginOverlap(TriggerGreen)
  (params (OverlappedComponent :type Primitive%20Component%20Object%20Reference) (OtherActor :type Actor%20Object%20Reference) (OtherComp :type Primitive%20Component%20Object%20Reference) (OtherBodyIndex :type Integer) (bFromSweep :type Boolean) (SweepResult :type Hit%20Result%20Structure%20%28by%20ref%29))
  (if (Variables|Default|GetisOn)
    (if (not (Variables|Default|GetBlocPlayer))
      (for _array_element (Variables|Default|GetaK_aRRAY)
        (Class|AkComponent|PostAkEvent _array_element "/Game/AudioEvents/Wall_Green_Through.Wall_Green_Through")))))

(event Custom|CustomTurnOn
  (bind _staticmesh (Variables|Default|GetStaticMesh))
  (bind _staticmesh_2 (Variables|Default|GetStaticMesh))
  (Variables|Default|SetisOn true)
  (Collision|SetCollisionEnabled _staticmesh_2 "QueryAndPhysics")
  (Development|SetHiddeninGame _staticmesh_2 false false)
  (if (Variables|Default|GetBlocPlayer)
    (Rendering|SetVisibility _staticmesh true false)
    (Collision|SetCollisionEnabled (Variables|Default|GetStaticMesh) "QueryAndPhysics")
    (Collision|SetCollisionResponsetoChannel _staticmesh "ECC_Pawn" "ECR_Block")
    (Collision|SetCollisionResponsetoChannel _staticmesh "ECC_GameTraceChannel1" "ECR_Ignore")
    (Collision|SetCollisionResponsetoChannel _staticmesh "ECC_GameTraceChannel4" "ECR_Ignore")
    (Collision|SetCollisionResponsetoChannel _staticmesh "ECC_GameTraceChannel9" "ECR_Ignore")
    (else
      (Rendering|SetVisibility _staticmesh true false)
      (Collision|SetCollisionEnabled (Variables|Default|GetStaticMesh) "QueryAndPhysics")
      (Collision|SetCollisionResponsetoChannel _staticmesh "ECC_Pawn" "ECR_Ignore")
      (Collision|SetCollisionResponsetoChannel _staticmesh "ECC_GameTraceChannel1" "ECR_Block")
      (Collision|SetCollisionResponsetoChannel _staticmesh "ECC_GameTraceChannel4" "ECR_Block")
      (Collision|SetCollisionResponsetoChannel _staticmesh "ECC_GameTraceChannel9" "ECR_Block"))))

(event Custom|ChangetoBlocTir
  (bind _staticmesh (Variables|Default|GetStaticMesh))
  (Variables|Default|SetBlocPlayer false)
  (Collision|SetCollisionResponsetoChannel _staticmesh "ECC_Pawn" "ECR_Ignore")
  (Collision|SetCollisionResponsetoChannel _staticmesh "ECC_GameTraceChannel1" "ECR_Block")
  (Collision|SetCollisionResponsetoChannel _staticmesh "ECC_GameTraceChannel4" "ECR_Block")
  (Rendering|Material|SetMaterial _staticmesh 0 "/Game/SecondaryMecanic/Bloc/Mat_Ins_BlocTir.Mat_Ins_BlocTir")
  (Collision|SetCollisionResponsetoChannel _staticmesh "ECC_GameTraceChannel9" "ECR_Block"))

(event Custom|TunrOn
  (bind _staticmesh (Variables|Default|GetStaticMesh))
  (bind _staticmesh_2 (Variables|Default|GetStaticMesh))
  (bind _staticmesh_3 (Variables|Default|GetStaticMesh))
  (bind _staticmesh_4 (Variables|Default|GetStaticMesh))
  (Rendering|SetVisibility (Variables|Default|GetStaticMesh) true true)
  (Variables|Default|SetisOn true)
  (if (Variables|Default|GetBlocPlayer)
    (if (Variables|Default|GetisMovable)
      (Collision|SetCollisionResponsetoChannel (Variables|Default|GetStaticMesh) "ECC_Pawn" "ECR_Block")
      (Collision|SetCollisionResponsetoChannel _staticmesh "ECC_GameTraceChannel1" "ECR_Ignore")
      (Collision|SetCollisionResponsetoChannel _staticmesh "ECC_GameTraceChannel4" "ECR_Ignore")
      (Rendering|Material|SetMaterial _staticmesh 0 "/Game/SecondaryMecanic/Bloc/Mat_Ins_BlocJoueur_Mov.Mat_Ins_BlocJoueur_Mov")
      (Collision|SetCollisionResponsetoChannel _staticmesh "ECC_GameTraceChannel9" "ECR_Ignore")
      (elif (Variables|Default|GetisDeactivable)
        (Collision|SetCollisionResponsetoChannel _staticmesh_3 "ECC_Pawn" "ECR_Block")
        (Collision|SetCollisionResponsetoChannel _staticmesh_3 "ECC_GameTraceChannel1" "ECR_Ignore")
        (Collision|SetCollisionResponsetoChannel _staticmesh_3 "ECC_GameTraceChannel4" "ECR_Ignore")
        (Rendering|Material|SetMaterial _staticmesh_3 0 "/Game/SecondaryMecanic/Bloc/Mat_Ins_BlocJoueurIns_Deac.Mat_Ins_BlocJoueurIns_Deac")
        (Collision|SetCollisionResponsetoChannel _staticmesh_3 "ECC_GameTraceChannel9" "ECR_Ignore")
        (for _array_element (Variables|Default|GetaK_aRRAY)
          (Class|AkComponent|PostAkEvent _array_element "/Game/AudioEvents/Wall_Amb.Wall_Amb"))
        (else
          (Collision|SetCollisionResponsetoChannel _staticmesh_3 "ECC_Pawn" "ECR_Block")
          (Collision|SetCollisionResponsetoChannel _staticmesh_3 "ECC_GameTraceChannel1" "ECR_Ignore")
          (Collision|SetCollisionResponsetoChannel _staticmesh_3 "ECC_GameTraceChannel4" "ECR_Ignore")
          (Rendering|Material|SetMaterial _staticmesh_3 0 "/Game/SecondaryMecanic/Bloc/Mat_Ins_BlocJouerIns.Mat_Ins_BlocJouerIns")
          (Collision|SetCollisionResponsetoChannel _staticmesh_3 "ECC_GameTraceChannel9" "ECR_Ignore")
          (if (not (Variables|Default|GetisOn))
            (Utilities|FlowControl|Delay 0.2)
            (Development|PrintString "stop3")
            (Class|AkComponent|Stop (Variables|Default|GetWall_Amb))
            (if (not (Variables|Default|GetisOn))
              (Collision|SetCollisionEnabled _staticmesh_4 "NoCollision")
              (Development|SetHiddeninGame _staticmesh_4 true false)
              (Development|PrintString "turnOFFF" true true "(R=1.000000,G=0.000000,B=0.577069,A=1.000000)" 1e+01)
              (Development|PrintString "stop4")
              (Class|AkComponent|Stop (Variables|Default|GetWall_Amb)))))))
    (elif (Variables|Default|GetisMovable)
      (Collision|SetCollisionResponsetoChannel _staticmesh_3 "ECC_Pawn" "ECR_Ignore")
      (Collision|SetCollisionResponsetoChannel _staticmesh_3 "ECC_GameTraceChannel1" "ECR_Block")
      (Collision|SetCollisionResponsetoChannel _staticmesh_3 "ECC_GameTraceChannel4" "ECR_Block")
      (Rendering|Material|SetMaterial _staticmesh_3 0 "/Game/SecondaryMecanic/Bloc/Mat_Ins_BlocTir_Mov.Mat_Ins_BlocTir_Mov")
      (Collision|SetCollisionResponsetoChannel _staticmesh_3 "ECC_GameTraceChannel9" "ECR_Block")
      (elif (Variables|Default|GetisDeactivable)
        (Collision|SetCollisionResponsetoChannel _staticmesh_2 "ECC_Pawn" "ECR_Ignore")
        (Collision|SetCollisionResponsetoChannel _staticmesh_2 "ECC_GameTraceChannel1" "ECR_Block")
        (Collision|SetCollisionResponsetoChannel _staticmesh_2 "ECC_GameTraceChannel4" "ECR_Block")
        (Rendering|Material|SetMaterial _staticmesh_2 0 "/Game/SecondaryMecanic/Bloc/Mat_Ins_BlocTir_Deac.Mat_Ins_BlocTir_Deac")
        (Collision|SetCollisionResponsetoChannel _staticmesh_2 "ECC_GameTraceChannel9" "ECR_Block")
        (for _array_element_2 (Variables|Default|GetaK_aRRAY)
          (Class|AkComponent|PostAkEvent _array_element_2 "/Game/AudioEvents/Wall_Amb.Wall_Amb"))
        (else
          (Collision|SetCollisionResponsetoChannel _staticmesh_2 "ECC_Pawn" "ECR_Ignore")
          (Collision|SetCollisionResponsetoChannel _staticmesh_2 "ECC_GameTraceChannel1" "ECR_Block")
          (Collision|SetCollisionResponsetoChannel _staticmesh_2 "ECC_GameTraceChannel4" "ECR_Block")
          (Rendering|Material|SetMaterial _staticmesh_2 0 "/Game/SecondaryMecanic/Bloc/Mat_Ins_BlocTir.Mat_Ins_BlocTir")
          (Collision|SetCollisionResponsetoChannel _staticmesh_2 "ECC_GameTraceChannel9" "ECR_Block"))))))

(event Custom|TurnOff
  (bind _staticmesh (Variables|Default|GetStaticMesh))
  (Variables|Default|SetisOn false)
  (Collision|SetCollisionEnabled _staticmesh "NoCollision")
  (Development|PrintString "testWall" true true "(R=0.000000,G=0.660000,B=1.000000,A=1.000000)" 5.0)
  (Rendering|SetVisibility _staticmesh false false))

(event Custom|ChangeToBlocJoueur
  (bind _staticmesh (Variables|Default|GetStaticMesh))
  (Variables|Default|SetBlocPlayer true)
  (Collision|SetCollisionResponsetoChannel _staticmesh "ECC_Pawn" "ECR_Block")
  (Collision|SetCollisionResponsetoChannel _staticmesh "ECC_GameTraceChannel1" "ECR_Ignore")
  (Collision|SetCollisionResponsetoChannel _staticmesh "ECC_GameTraceChannel4" "ECR_Ignore")
  (Rendering|Material|SetMaterial _staticmesh 0 "/Game/SecondaryMecanic/Bloc/Mat_Ins_BlocJouerIns.Mat_Ins_BlocJouerIns")
  (Collision|SetCollisionResponsetoChannel _staticmesh "ECC_GameTraceChannel9" "ECR_Ignore"))

(event EventBeginPlay
  (bind _staticmesh (Variables|Default|GetStaticMesh))
  (bind _ison (Variables|Default|GetisOn))
  (bind _staticmesh_2 (Variables|Default|GetStaticMesh))
  (bind _staticmesh_3 (Variables|Default|GetStaticMesh))
  (bind _staticmesh_4 (Variables|Default|GetStaticMesh))
  (Variables|Default|SetaK_aRRAY (Utilities|Array|MakeArray (Variables|Default|GetAk3) (Variables|Default|GetAk) (Variables|Default|GetAk1) (Variables|Default|GetAk2) (Variables|Default|GetWall_Amb) (Variables|Default|GetAk4) (Variables|Default|GetAk5) (Variables|Default|GetAk6) (Variables|Default|GetAk7)))
  (if (Variables|Default|GetBlocPlayer)
    (if (Variables|Default|GetisMovable)
      (Collision|SetCollisionResponsetoChannel (Variables|Default|GetStaticMesh) "ECC_Pawn" "ECR_Block")
      (Collision|SetCollisionResponsetoChannel _staticmesh "ECC_GameTraceChannel1" "ECR_Ignore")
      (Collision|SetCollisionResponsetoChannel _staticmesh "ECC_GameTraceChannel4" "ECR_Ignore")
      (Rendering|Material|SetMaterial _staticmesh 0 "/Game/SecondaryMecanic/Bloc/Mat_Ins_BlocJoueur_Mov.Mat_Ins_BlocJoueur_Mov")
      (Collision|SetCollisionResponsetoChannel _staticmesh "ECC_GameTraceChannel9" "ECR_Ignore")
      (elif (Variables|Default|GetisDeactivable)
        (Collision|SetCollisionResponsetoChannel _staticmesh_3 "ECC_Pawn" "ECR_Block")
        (Collision|SetCollisionResponsetoChannel _staticmesh_3 "ECC_GameTraceChannel1" "ECR_Ignore")
        (Collision|SetCollisionResponsetoChannel _staticmesh_3 "ECC_GameTraceChannel4" "ECR_Ignore")
        (Rendering|Material|SetMaterial _staticmesh_3 0 "/Game/SecondaryMecanic/Bloc/Mat_Ins_BlocJoueurIns_Deac.Mat_Ins_BlocJoueurIns_Deac")
        (Collision|SetCollisionResponsetoChannel _staticmesh_3 "ECC_GameTraceChannel9" "ECR_Ignore")
        (for _array_element (Variables|Default|GetaK_aRRAY)
          (Class|AkComponent|PostAkEvent _array_element "/Game/AudioEvents/Wall_Amb.Wall_Amb"))
        (else
          (Collision|SetCollisionResponsetoChannel _staticmesh_3 "ECC_Pawn" "ECR_Block")
          (Collision|SetCollisionResponsetoChannel _staticmesh_3 "ECC_GameTraceChannel1" "ECR_Ignore")
          (Collision|SetCollisionResponsetoChannel _staticmesh_3 "ECC_GameTraceChannel4" "ECR_Ignore")
          (Rendering|Material|SetMaterial _staticmesh_3 0 "/Game/SecondaryMecanic/Bloc/Mat_Ins_BlocJouerIns.Mat_Ins_BlocJouerIns")
          (Collision|SetCollisionResponsetoChannel _staticmesh_3 "ECC_GameTraceChannel9" "ECR_Ignore")
          (if (not _ison)
            (Utilities|FlowControl|Delay 0.2)
            (Development|PrintString "stop3")
            (Class|AkComponent|Stop (Variables|Default|GetWall_Amb))
            (if (not _ison)
              (Collision|SetCollisionEnabled _staticmesh_4 "NoCollision")
              (Development|SetHiddeninGame _staticmesh_4 true false)
              (Development|PrintString "turnOFFF" true true "(R=1.000000,G=0.000000,B=0.577069,A=1.000000)" 1e+01)
              (Development|PrintString "stop4")
              (Class|AkComponent|Stop (Variables|Default|GetWall_Amb)))))))
    (elif (Variables|Default|GetisMovable)
      (Collision|SetCollisionResponsetoChannel _staticmesh_3 "ECC_Pawn" "ECR_Ignore")
      (Collision|SetCollisionResponsetoChannel _staticmesh_3 "ECC_GameTraceChannel1" "ECR_Block")
      (Collision|SetCollisionResponsetoChannel _staticmesh_3 "ECC_GameTraceChannel4" "ECR_Block")
      (Rendering|Material|SetMaterial _staticmesh_3 0 "/Game/SecondaryMecanic/Bloc/Mat_Ins_BlocTir_Mov.Mat_Ins_BlocTir_Mov")
      (Collision|SetCollisionResponsetoChannel _staticmesh_3 "ECC_GameTraceChannel9" "ECR_Block")
      (elif (Variables|Default|GetisDeactivable)
        (Collision|SetCollisionResponsetoChannel _staticmesh_2 "ECC_Pawn" "ECR_Ignore")
        (Collision|SetCollisionResponsetoChannel _staticmesh_2 "ECC_GameTraceChannel1" "ECR_Block")
        (Collision|SetCollisionResponsetoChannel _staticmesh_2 "ECC_GameTraceChannel4" "ECR_Block")
        (Rendering|Material|SetMaterial _staticmesh_2 0 "/Game/SecondaryMecanic/Bloc/Mat_Ins_BlocTir_Deac.Mat_Ins_BlocTir_Deac")
        (Collision|SetCollisionResponsetoChannel _staticmesh_2 "ECC_GameTraceChannel9" "ECR_Block")
        (for _array_element_2 (Variables|Default|GetaK_aRRAY)
          (Class|AkComponent|PostAkEvent _array_element_2 "/Game/AudioEvents/Wall_Amb.Wall_Amb"))
        (else
          (Collision|SetCollisionResponsetoChannel _staticmesh_2 "ECC_Pawn" "ECR_Ignore")
          (Collision|SetCollisionResponsetoChannel _staticmesh_2 "ECC_GameTraceChannel1" "ECR_Block")
          (Collision|SetCollisionResponsetoChannel _staticmesh_2 "ECC_GameTraceChannel4" "ECR_Block")
          (Rendering|Material|SetMaterial _staticmesh_2 0 "/Game/SecondaryMecanic/Bloc/Mat_Ins_BlocTir.Mat_Ins_BlocTir")
          (Collision|SetCollisionResponsetoChannel _staticmesh_2 "ECC_GameTraceChannel9" "ECR_Block"))))))

(event Collision|EventActorBeginOverlap
  (params (OtherActor :type Actor%20Object%20Reference)))

(event EventTick
  (params (DeltaSeconds :type Float%20%28single-precision%29)))

(fn ConstructionScript
  (bind _staticmesh (Variables|Default|GetStaticMesh))
  (bind _staticmesh_2 (Variables|Default|GetStaticMesh))
  (bind _staticmesh_3 (Variables|Default|GetStaticMesh))
  (bind _staticmesh_4 (Variables|Default|GetStaticMesh))
  (if (Variables|Default|GetisOn)
    (if (Variables|Default|GetBlocPlayer)
      (Class|AkGameplayStatics|SetSwitch "Wall_Amb" "Blue" (Components|GetOwner (Variables|Default|GetWall_Amb)))
      (if (Variables|Default|GetisMovable)
        (Class|AkComponent|PostAkEvent (Variables|Default|GetWall_Amb))
        (Collision|SetCollisionResponsetoChannel (Variables|Default|GetStaticMesh) "ECC_Pawn" "ECR_Block")
        (Collision|SetCollisionResponsetoChannel _staticmesh "ECC_GameTraceChannel1" "ECR_Ignore")
        (Collision|SetCollisionResponsetoChannel _staticmesh "ECC_GameTraceChannel4" "ECR_Ignore")
        (Rendering|Material|SetMaterial _staticmesh 0 "/Game/SecondaryMecanic/Bloc/Mat_Ins_BlocJoueur_Mov.Mat_Ins_BlocJoueur_Mov")
        (Collision|SetCollisionResponsetoChannel _staticmesh "ECC_GameTraceChannel9" "ECR_Ignore")
        (elif (Variables|Default|GetisDeactivable)
          (Collision|SetCollisionResponsetoChannel _staticmesh_3 "ECC_Pawn" "ECR_Block")
          (Collision|SetCollisionResponsetoChannel _staticmesh_3 "ECC_GameTraceChannel1" "ECR_Ignore")
          (Collision|SetCollisionResponsetoChannel _staticmesh_3 "ECC_GameTraceChannel4" "ECR_Ignore")
          (Rendering|Material|SetMaterial _staticmesh_3 0 "/Game/SecondaryMecanic/Bloc/Mat_Ins_BlocJoueurIns_Deac.Mat_Ins_BlocJoueurIns_Deac")
          (Collision|SetCollisionResponsetoChannel _staticmesh_3 "ECC_GameTraceChannel9" "ECR_Ignore")
          (Class|AkComponent|PostAkEvent (Variables|Default|GetWall_Amb))
          (else
            (Class|AkComponent|PostAkEvent (Variables|Default|GetWall_Amb))
            (Collision|SetCollisionResponsetoChannel _staticmesh_3 "ECC_Pawn" "ECR_Block")
            (Collision|SetCollisionResponsetoChannel _staticmesh_3 "ECC_GameTraceChannel1" "ECR_Ignore")
            (Collision|SetCollisionResponsetoChannel _staticmesh_3 "ECC_GameTraceChannel4" "ECR_Ignore")
            (Rendering|Material|SetMaterial _staticmesh_3 0 "/Game/SecondaryMecanic/Bloc/Mat_Ins_BlocJouerIns.Mat_Ins_BlocJouerIns")
            (Collision|SetCollisionResponsetoChannel _staticmesh_3 "ECC_GameTraceChannel9" "ECR_Ignore"))))
      (else
        (Class|AkGameplayStatics|SetSwitch "Wall_Amb" "Green" (Components|GetOwner (Variables|Default|GetWall_Amb)))
        (if (Variables|Default|GetisMovable)
          (Class|AkComponent|PostAkEvent (Variables|Default|GetWall_Amb))
          (Collision|SetCollisionResponsetoChannel _staticmesh_3 "ECC_Pawn" "ECR_Ignore")
          (Collision|SetCollisionResponsetoChannel _staticmesh_3 "ECC_GameTraceChannel1" "ECR_Block")
          (Collision|SetCollisionResponsetoChannel _staticmesh_3 "ECC_GameTraceChannel4" "ECR_Block")
          (Rendering|Material|SetMaterial _staticmesh_3 0 "/Game/SecondaryMecanic/Bloc/Mat_Ins_BlocTir_Mov.Mat_Ins_BlocTir_Mov")
          (Collision|SetCollisionResponsetoChannel _staticmesh_3 "ECC_GameTraceChannel9" "ECR_Block")
          (elif (Variables|Default|GetisDeactivable)
            (Collision|SetCollisionResponsetoChannel _staticmesh_2 "ECC_Pawn" "ECR_Ignore")
            (Collision|SetCollisionResponsetoChannel _staticmesh_2 "ECC_GameTraceChannel1" "ECR_Block")
            (Collision|SetCollisionResponsetoChannel _staticmesh_2 "ECC_GameTraceChannel4" "ECR_Block")
            (Rendering|Material|SetMaterial _staticmesh_2 0 "/Game/SecondaryMecanic/Bloc/Mat_Ins_BlocTir_Deac.Mat_Ins_BlocTir_Deac")
            (Collision|SetCollisionResponsetoChannel _staticmesh_2 "ECC_GameTraceChannel9" "ECR_Block")
            (else
              (Class|AkComponent|PostAkEvent (Variables|Default|GetWall_Amb))
              (Collision|SetCollisionResponsetoChannel _staticmesh_2 "ECC_Pawn" "ECR_Ignore")
              (Collision|SetCollisionResponsetoChannel _staticmesh_2 "ECC_GameTraceChannel1" "ECR_Block")
              (Collision|SetCollisionResponsetoChannel _staticmesh_2 "ECC_GameTraceChannel4" "ECR_Block")
              (Rendering|Material|SetMaterial _staticmesh_2 0 "/Game/SecondaryMecanic/Bloc/Mat_Ins_BlocTir.Mat_Ins_BlocTir")
              (Collision|SetCollisionResponsetoChannel _staticmesh_2 "ECC_GameTraceChannel9" "ECR_Block"))))))
    (else
      (Development|SetHiddeninGame _staticmesh_4 true false)
      (Collision|SetCollisionResponsetoAllChannels _staticmesh_4 "ECR_Ignore")
      (Development|PrintString "stop 5")
      (Class|AkComponent|Stop (Variables|Default|GetWall_Amb)))))