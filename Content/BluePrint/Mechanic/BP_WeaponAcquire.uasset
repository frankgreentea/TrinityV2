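; BP_WeaponAcquire is a glowing prop with animated-looking water materials, apparently marking a weapon acquisition point; it contains no pickup logic itself.
; The construction script applies exposed color and glow variables to both meshes' materials and the point light.
; BeginPlay unhides the actor, disables tick and starts the Globe's Wwise audio.
; ShutDown destroys the light and Globe, then dims the wave colors and glow to leave it spent.
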(event Custom|ShutDown
  (Components|DestroyComponent (Variables|Default|GetPointLight))
  (Rendering|Material|SetVectorParameterValueonMaterials (Variables|Debug|GetStaticMeshComponent) "Wave Base Color" "0.100000,0.100000,0.100000")
  (Rendering|Material|SetScalarParameterValueonMaterials (Variables|Debug|GetStaticMeshComponent) "glow" 0.1)
  (Rendering|Material|SetVectorParameterValueonMaterials (Variables|Debug|GetStaticMeshComponent) "Wave Crest Color" "0.100000,0.100000,0.100000"))

(event EventBeginPlay
  (Rendering|SetActorHiddenInGame false)
  (Actor|Tick|SetActorTickEnabled false)
  (Class|AkComponent|PostAssociatedAkEvent (Variables|Default|GetGlobe)))

(event Collision|EventActorBeginOverlap
  (params (OtherActor :type Actor%20Object%20Reference)))

(fn ConstructionScript
  (Rendering|Material|SetScalarParameterValueonMaterials (Variables|Debug|GetStaticMeshComponent) "glow" (Variables|Default|Getglow))
  (Rendering|Material|SetVectorParameterValueonMaterials (Variables|Debug|GetStaticMeshComponent) "linecolor" (Variables|Default|Getcolorline))
  (Rendering|Material|SetVectorParameterValueonMaterials (Variables|Debug|GetStaticMeshComponent) "Wave Base Color" (Variables|Default|GetcolorWater))
  (Rendering|Material|SetScalarParameterValueonMaterials (Variables|Debug|GetStaticMeshComponent) "glow" (Variables|Default|Getglowwater))
  (Rendering|Components|Light|SetLightColor (Variables|Default|GetPointLight) (Variables|Default|GetlightColor) true)
  (Rendering|Material|SetVectorParameterValueonMaterials (Variables|Debug|GetStaticMeshComponent) "Wave Crest Color" (Variables|Default|GetCrestColor)))