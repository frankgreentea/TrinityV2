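; Weapon grab/drop point that changes the player character's WeaponType when overlapped.
; BeginPlay tints its meshes, choosing a yellow, red or blue emissive color from the ChangeTo flags.
; Each overlap plays a Wwise Grab or Drop sound based on KeepWeapon.
; If the player's WeaponType matches, it steps that type up or down along the yellow or non-yellow path, refreshes the crosshair and flips KeepWeapon.
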(event EventBeginPlay
  (Rendering|Material|SetVectorParameterValueonMaterials (Variables|Default|GetCube) "Base Color" (Variables|Default|GetColor))
  (if (Variables|Default|GetchangeToYellow)
    (Rendering|Material|SetVectorParameterValueonMaterials (Variables|Default|GetCube1) "Emissive Color" (Variables|Default|GetYellowColor))
    (elif (Variables|Default|GetchangeToRed)
      (Rendering|Material|SetVectorParameterValueonMaterials (Variables|Default|GetCube1) "Emissive Color" (Variables|Default|GetredColor))
      (else
        (Rendering|Material|SetVectorParameterValueonMaterials (Variables|Default|GetCube1) "Emissive Color" (Variables|Default|GetBlueColor))))))

(event Collision|EventActorBeginOverlap
  (params (OtherActor :type Actor%20Object%20Reference))
  (bind _returnvalue (Game|GetPlayerCharacter 0))
  (bind _returnvalue_2 (Game|GetPlayerCharacter 0))
  (bind _returnvalue_3 (Game|GetPlayerCharacter 0))
  (if (Variables|Default|GetKeepWeapon)
    (Class|AkGameplayStatics|SetSwitch "Door" "Drop" _returnvalue_2)
    (Class|AkGameplayStatics|PostEvent "/Game/AudioEvents/Door.Door" _returnvalue_2 false)
    (if (Variables|Default|GetchangeToYellow)
      (bind _asbp_my_character (Utilities|Casting|CastToBP_MyCharacter (Game|GetPlayerCharacter 0)))
      (switch int (Variables|/Game/BaseGame/BP_MyCharacter.BP_MyCharacter_C|GetWeaponType _asbp_my_character)
        (:5
          (bind _asbp_my_character_2 (Utilities|Casting|CastToBP_MyCharacter (Game|GetPlayerCharacter 0)))
          (Default|NormalCrossHairSetup _asbp_my_character_2)
          (Variables|/Game/BaseGame/BP_MyCharacter.BP_MyCharacter_C|SetWeaponType _asbp_my_character 4)
          (Variables|Default|SetKeepWeapon false)))
      (else
        (bind _asbp_my_character_3 (Utilities|Casting|CastToBP_MyCharacter (Game|GetPlayerCharacter 0)))
        (switch int (Variables|/Game/BaseGame/BP_MyCharacter.BP_MyCharacter_C|GetWeaponType _asbp_my_character_3)
          (:4
            (bind _asbp_my_character_4 (Utilities|Casting|CastToBP_MyCharacter (Game|GetPlayerCharacter 0)))
            (Default|OnlyBlue _asbp_my_character_4)
            (Variables|/Game/BaseGame/BP_MyCharacter.BP_MyCharacter_C|SetWeaponType _asbp_my_character_3 1)
            (Variables|Default|SetKeepWeapon false)))))
    (else
      (Class|AkGameplayStatics|SetSwitch "Door" "Grab" _returnvalue_3)
      (Class|AkGameplayStatics|PostEvent "/Game/AudioEvents/Door.Door" _returnvalue_3 false)
      (if (Variables|Default|GetchangeToYellow)
        (bind _asbp_my_character_5 (Utilities|Casting|CastToBP_MyCharacter _returnvalue))
        (switch int (Variables|/Game/BaseGame/BP_MyCharacter.BP_MyCharacter_C|GetWeaponType _asbp_my_character_5)
          (:4
            (bind _asbp_my_character_6 (Utilities|Casting|CastToBP_MyCharacter (Game|GetPlayerCharacter 0)))
            (Default|NormalCrossHairSetup _asbp_my_character_6)
            (Variables|/Game/BaseGame/BP_MyCharacter.BP_MyCharacter_C|SetWeaponType _asbp_my_character_5 5)
            (Variables|Default|SetKeepWeapon true)))
        (else
          (bind _asbp_my_character_7 (Utilities|Casting|CastToBP_MyCharacter _returnvalue))
          (switch int (Variables|/Game/BaseGame/BP_MyCharacter.BP_MyCharacter_C|GetWeaponType _asbp_my_character_7)
            (:1
              (bind _asbp_my_character_8 (Utilities|Casting|CastToBP_MyCharacter (Game|GetPlayerCharacter 0)))
              (Default|NormalCrossHairSetup _asbp_my_character_8)
              (Variables|/Game/BaseGame/BP_MyCharacter.BP_MyCharacter_C|SetWeaponType _asbp_my_character_7 4)
              (Variables|Default|SetKeepWeapon true))))))))

(event EventTick
  (params (DeltaSeconds :type Float%20%28single-precision%29)))

(fn ConstructionScript)