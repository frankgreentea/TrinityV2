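; Pyramid actor that glows blue, red or yellow by its shot type (optionally randomized) and plays Wwise shooting audio.
; For red and yellow types, beamevent spawns attraction particles and sets per-pyramid colors in a material parameter collection.
; Two chained timelines loop particle scale and base glow, with a play rate derived from ShootDelay.
; When active, electric arcs track the target Prism_BP's cart through a 0.2-second Delay loop.
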(event Custom|shutdown
  (Rendering|Material|SetScalarParameterValueonMaterials (Variables|Default|Getbase) "Glow" 0.1))

(event Custom|randomassigne
  (Variables|Default|SetTirNumber (Math|Random|RandomIntegerinRange 1 3))
  (Variables|Default|SetrandomDelau (Math|Random|RandomFloatinRange 1.0 6.0)))

(event Custom|ShootPyr
  (Class|AkGameplayStatics|PostEvent "/Game/AudioEvents/Pyramid_Shoot.Pyramid_Shoot" self))

(event Custom|RestOfTiimelinme
  (bind _newtrack_3 (Timeline|Timeline_1 PlayFromStart)
    (:Update
      (Rendering|Material|SetScalarParameterValueonMaterials (Variables|Default|Getbase) "Glow" _newtrack_3))
    (:Finished
      (CallFunction|AttractionParticuleTimeron))))

(event Custom|StartUp
  (Utilities|FlowControl|Delay (Variables|Default|GetrandomDelau))
  (Rendering|Material|SetScalarParameterValueonMaterials (Variables|Default|Getbase) "Glow" 2e+01))

(event Custom|ActivateTimer
  (CallFunction|AttractionParticuleTimeron))

(event Custom|AttractionParticuleTimerOn
  (bind _newtrack_1 (Timeline|Timeline_0 PlayFromStart)
    (:Update
      (Transformation|SetWorldScale3D (Variables|Default|GetAttractionPart) (Math|Vector|MakeVector _newtrack_1 _newtrack_1 _newtrack_1)))
    (:Finished
      (CallFunction|RestOfTiimelinme))))

(event Custom|beamevent
  (bind _cubecc (Variables|Default|GetCubecc))
  (bind _active (Variables|Default|Getactive))
  (bind _returnvalue (Transformation|GetWorldLocation _cubecc))
  (Development|PrintString "Step1" false true "(R=1.000000,G=0.014359,B=0.000000,A=1.000000)" 1e+01)
  (switch int (Variables|Default|GetTirNumber)
    (:2
      (switch int (Variables|Default|GetPyrNumber)
        (:0
          (Rendering|Material|SetVectorParameterValue "/Game/Particle/PyramidTrail/sparkOne_Coll.sparkOne_Coll" "Colorpyr1" (Utilities|Struct|MakeLinearColor 1.0 0.1 0.1 1.0) :!class /Script/Engine.KismetMaterialLibrary)
          (bind _returnvalue_2 (Effects|SpawnEmitterAttached "/Game/Particle/PyramidTrail/P_GPU_particles_attraction.P_GPU_particles_attraction" (Variables|Default|GetCubecc) "None" "0, 0, 0" "0.000000, 0, 0" "1.000000,1.000000,1.000000" "SnapToTargetIncludingScale" :!label _label))
          (Variables|Default|SetAttractionPart _returnvalue_2)
          (Transformation|SetWorldScale3D _returnvalue_2 "0.900000,0.900000,0.900000")
          (CallFunction|ActivateTimer)
          (Components|Timeline|SetPlayRate (Variables|Default|GetTimeline_0) (/ 1.0 (- (Variables|Default|GetShootDelay) 0.6)))
          (if _active
            (Development|PrintString "Hello" false)
            (bind _returnvalue_3 (Effects|SpawnEmitterAttached "/Game/Particle/PyramidTrail/P_electricity_arc.P_electricity_arc" _cubecc "None" "0, 0, 0" "0.000000, 0, 0" "1.000000,1.000000,1.000000" "SnapToTarget"))
            (if _active :!label _label_2
              (bind _asprism_bp (Utilities|Casting|CastToPrism_BP (Variables|Default|GetpyramidActor_target)))
              (Class|ParticleSystemComponent|SetBeamSourcePoint _returnvalue_3 0 _returnvalue)
              (Class|ParticleSystemComponent|SetBeamSourcePoint _returnvalue_3 2 _returnvalue)
              (Class|ParticleSystemComponent|SetBeamTargetPoint _returnvalue_3 2 (Transformation|GetWorldLocation (Variables|/Game/BluePrint/Mechanic/Prism_BP.Prism_BP_C|GetCart _asprism_bp)))
              (Class|ParticleSystemComponent|SetBeamTargetPoint _returnvalue_3 0 (Transformation|GetWorldLocation (Variables|/Game/BluePrint/Mechanic/Prism_BP.Prism_BP_C|GetCart _asprism_bp)))
              (Development|PrintString (Utilities|String|ToString(Vector) (Transformation|GetWorldLocation _returnvalue_3)) false)
              (Utilities|FlowControl|Delay 0.2)
              (goto _label_2))))
        (:1
          (Rendering|Material|SetVectorParameterValue "/Game/Particle/PyramidTrail/sparkOne_Coll.sparkOne_Coll" "ColorPyr2" (Utilities|Struct|MakeLinearColor 1.0 0.1 0.1 1.0) :!class /Script/Engine.KismetMaterialLibrary)
          (bind _returnvalue_4 (Effects|SpawnEmitterAttached "/Game/Particle/PyramidTrail/P_GPU_particles_attraction_2.P_GPU_particles_attraction_2" (Variables|Default|GetCubecc) "None" "0, 0,0.000000" "0, 0, 0" "1.000000,1.000000,1.000000" "SnapToTarget" :!label _label_3))
          (Variables|Default|SetAttractionPart _returnvalue_4)
          (Transformation|SetWorldScale3D _returnvalue_4 "0.900000,0.900000,0.900000")
          (CallFunction|ActivateTimer)
          (Components|Timeline|SetPlayRate (Variables|Default|GetTimeline_0) (/ 1.0 (- (Variables|Default|GetShootDelay) 0.6)))
          (if (Variables|Default|Getactive)
            (bind _returnvalue_5 (Effects|SpawnEmitterAttached "/Game/Particle/PyramidTrail/P_electricity_arc_pyr2.P_electricity_arc_pyr2" (Variables|Default|GetCubecc) "None" "0,0.000000, 0" "0, 0, 0" "1.000000,1.000000,1.000000" "SnapToTarget"))
            (bind _asprism_bp_2 (Utilities|Casting|CastToPrism_BP (Variables|Default|GetpyramidActor_target) :!label _label_4))
            (Class|ParticleSystemComponent|SetBeamTargetPoint _returnvalue_5 2 (Transformation|GetWorldLocation (Variables|/Game/BluePrint/Mechanic/Prism_BP.Prism_BP_C|GetCart _asprism_bp_2)))
            (Class|ParticleSystemComponent|SetBeamTargetPoint _returnvalue_5 0 (Transformation|GetWorldLocation (Variables|/Game/BluePrint/Mechanic/Prism_BP.Prism_BP_C|GetCart _asprism_bp_2)))
            (Utilities|FlowControl|Delay 0.2)
            (Development|PrintString "electricart" false false)
            (goto _label_4)))
        (:2
          (Rendering|Material|SetVectorParameterValue "/Game/Particle/PyramidTrail/sparkOne_Coll.sparkOne_Coll" "ColorPyr3" (Utilities|Struct|MakeLinearColor 1.0 0.1 0.1 1.0) :!class /Script/Engine.KismetMaterialLibrary)
          (bind _returnvalue_6 (Effects|SpawnEmitterAttached "/Game/Particle/PyramidTrail/P_GPU_particles_attraction_3.P_GPU_particles_attraction_3" (Variables|Default|GetCubecc) "None" "0, 0, 0" "0.000000, 0, 0" "1.000000,1.000000,1.000000" "SnapToTargetIncludingScale" :!label _label_5))
          (Variables|Default|SetAttractionPart _returnvalue_6)
          (Transformation|SetWorldScale3D _returnvalue_6 "0.900000,0.900000,0.900000")
          (CallFunction|ActivateTimer)
          (Components|Timeline|SetPlayRate (Variables|Default|GetTimeline_0) (/ 1.0 (- (Variables|Default|GetShootDelay) 0.6)))
          (if (Variables|Default|Getactive)
            (bind _returnvalue_7 (Effects|SpawnEmitterAttached "/Game/Particle/PyramidTrail/P_electricity_arc_3.P_electricity_arc_3" (Variables|Default|GetCubecc) "None" "0,0.000000, 0" "0, 0, 0" "1.000000,1.000000,1.000000" "SnapToTarget"))
            (bind _asprism_bp_3 (Utilities|Casting|CastToPrism_BP (Variables|Default|GetpyramidActor_target) :!label _label_6))
            (Class|ParticleSystemComponent|SetBeamTargetPoint _returnvalue_7 2 (Transformation|GetWorldLocation (Variables|/Game/BluePrint/Mechanic/Prism_BP.Prism_BP_C|GetCart _asprism_bp_3)))
            (Class|ParticleSystemComponent|SetBeamTargetPoint _returnvalue_7 0 (Transformation|GetWorldLocation (Variables|/Game/BluePrint/Mechanic/Prism_BP.Prism_BP_C|GetCart _asprism_bp_3)))
            (Utilities|FlowControl|Delay 0.2)
            (goto _label_6)))))
    (:3
      (Development|PrintString "Step2" false)
      (switch int (Variables|Default|GetPyrNumber)
        (:0
          (goto _label))
        (:1
          (Rendering|Material|SetVectorParameterValue "/Game/Particle/PyramidTrail/sparkOne_Coll.sparkOne_Coll" "ColorPyr2" (Utilities|Struct|MakeLinearColor 1.0 1.0 0.0 1.0) :!class /Script/Engine.KismetMaterialLibrary)
          (goto _label_3))
        (:2
          (Rendering|Material|SetVectorParameterValue "/Game/Particle/PyramidTrail/sparkOne_Coll.sparkOne_Coll" "ColorPyr3" (Utilities|Struct|MakeLinearColor 1.0 1.0 0.0 1.0) :!class /Script/Engine.KismetMaterialLibrary)
          (goto _label_5))))))

(event EventBeginPlay
  (Class|AkGameplayStatics|SetRTPCValue "Pyramid" (Variables|Default|GetShootDelay) 0 self)
  (if (Variables|Default|GetrandomAssignement)
    (CallFunction|Randomassigne))
  (if (Variables|Default|GetstartClose)
    (Rendering|Material|SetScalarParameterValueonMaterials (Variables|Default|Getbase) "Glow" 0.1)
    (else
      (Rendering|Material|SetScalarParameterValueonMaterials (Variables|Default|Getbase) "Glow" 2e+01)))
  (switch int (Variables|Default|GetTirNumber)
    (:1
      (Rendering|Material|SetVectorParameterValueonMaterials (Variables|Default|Getbase) "Color" "0,0.300000,1.000000"))
    (:2
      (Rendering|Material|SetVectorParameterValueonMaterials (Variables|Default|Getbase) "Color" "1.000000, 0, 0"))
    (:3
      (Rendering|Material|SetVectorParameterValueonMaterials (Variables|Default|Getbase) "Color" "1.000000,0.800000, 0"))))

(event Collision|EventActorBeginOverlap
  (params (OtherActor :type Actor%20Object%20Reference)))

(event EventTick
  (params (DeltaSeconds :type Float%20%28single-precision%29)))

(fn ConstructionScript)