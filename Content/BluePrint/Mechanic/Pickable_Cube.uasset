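; Pickable physics cube that signals when it can be picked up or is held, and can respawn.
; Events raise or dim the material Glow parameter on the cube and its respawn component, and swap the cube to glass while held.
; Respawn zeroes physics velocity and moves the cube to the Scene component's location.
; Construction removes RespawnBorn when HasRespawnBorn is off; hits print the other actor's name.
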(event OnComponentHit(Cube)
  (params (HitComponent :type Primitive%20Component%20Object%20Reference) (OtherActor :type Actor%20Object%20Reference) (OtherComp :type Primitive%20Component%20Object%20Reference) (NormalImpulse :type Vector :default "0, 0, 0") (Hit :type Hit%20Result%20Structure%20%28by%20ref%29))
  (Development|PrintString (Utilities|GetDisplayName OtherActor)))

(event Custom|Cube_Respawn
  (Class|PrimitiveComponent|SetAllPhysicsLinearVelocity (Variables|Default|GetCube) "0, 0, 0" false)
  (Transformation|SetWorldLocation (Variables|Default|GetCube) (Transformation|GetWorldLocation (Variables|Default|GetScene)) false false))

(event Custom|RespawnBornInView
  (Rendering|Material|SetScalarParameterValueonMaterials (Variables|Default|GetRespawnBorn1) "Glow" 5e+01))

(event Custom|CanPickUp
  (Rendering|Material|SetScalarParameterValueonMaterials (Variables|Default|GetCube) "Glow" 5e+01))

(event Custom|CanNotPickUp
  (Rendering|Material|SetScalarParameterValueonMaterials (Variables|Default|GetCube) "Glow" 0.5))

(event Custom|Picked
  (Rendering|Material|SetMaterial (Variables|Default|GetCube) 0 "/Game/StarterContent/Materials/M_Glass_Inst.M_Glass_Inst"))

(event Custom|Release
  (Rendering|Material|SetMaterial (Variables|Default|GetCube) 0 "/Game/Materials/Mecanic/GlowBase_Inst.GlowBase_Inst"))

(event Custom|RespawnBornOutOfView
  (Rendering|Material|SetScalarParameterValueonMaterials (Variables|Default|GetRespawnBorn1) "Glow" 0.5))

(event EventBeginPlay)

(event Collision|EventActorBeginOverlap
  (params (OtherActor :type Actor%20Object%20Reference)))

(event EventTick
  (params (DeltaSeconds :type Float%20%28single-precision%29)))

(fn ConstructionScript
  (Rendering|Material|SetScalarParameterValueonMaterials (Variables|Default|GetCube) "Glow" 0.5)
  (if (not (Variables|Default|GetHasRespawnBorn))
    (Components|DestroyComponent (Variables|Default|GetRespawnBorn))))