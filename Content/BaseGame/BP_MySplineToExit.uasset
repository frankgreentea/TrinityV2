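; Temporary guide actor that draws a spline path from the player to the exit location, then destroys itself after five seconds.
; Shortly after BeginPlay, it moves the first two spline points to an offset from the player and to ExitPlace.
; Each segment gets two spline meshes on identical start and end data plus static mesh markers at both ends, all attached to Topview.
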(event EventBeginPlay
  (bind _returnvalue (Game|GetPlayerCharacter 0))
  (bind _topview (Variables|Default|Gettopview))
  (bind _topview_2 (Variables|Default|Gettopview))
  (bind _spline (Variables|Default|GetSpline))
  (bind _returnvalue_2 (Transformation|GetActorLocation _returnvalue))
  (Utilities|FlowControl|Delay 0.1)
  (Development|PrintString (Utilities|String|ToString(Vector) (Variables|Default|GetExitPlace)))
  (Spline|SetLocationatSplinePoint (Variables|Default|GetSpline) 0 (Math|Vector|MakeVector (+ (.x _returnvalue_2) 3e+01) (+ (.y _returnvalue_2) 3e+01) (+ (.z _returnvalue_2) 3e+01)) "World" false)
  (Spline|SetLocationatSplinePoint (Variables|Default|GetSpline) 1 (Variables|Default|GetExitPlace) "World" false)
  (for _index (range 0 (- (Spline|GetNumberOfSplinePoints _spline) 2))
    (bind _returnvalue_3 (AddComponent|AddSplineMeshComponent false))
    (Transformation|AttachComponentToComponent _returnvalue_3 _topview_2 "None" "KeepRelative" "KeepRelative" "KeepRelative" true)
    (SplineMesh|SetStartandEnd _returnvalue_3 (.Location (Spline|GetLocationandTangentatSplinePoint _spline _index "Local")) (.Tangent (Spline|GetLocationandTangentatSplinePoint _spline _index "Local")) (.Location (Spline|GetLocationandTangentatSplinePoint _spline (+ _index 1) "Local")) (.Tangent (Spline|GetLocationandTangentatSplinePoint _spline (+ _index 1) "Local")) true :!class /Script/Engine.SplineMeshComponent)
    (bind _returnvalue_4 (AddComponent|AddStaticMeshComponent false (Math|Transform|MakeTransform (.Location (Spline|GetLocationandTangentatSplinePoint _spline _index "Local")) "0, 0, 0" "0.700000,0.700000,0.700000")))
    (Transformation|AttachComponentToComponent _returnvalue_4 _topview "None" "KeepRelative" "KeepRelative" "KeepRelative" true)
    (bind _returnvalue_5 (AddComponent|AddStaticMeshComponent false (Math|Transform|MakeTransform (.Location (Spline|GetLocationandTangentatSplinePoint _spline (+ _index 1) "Local")) "0, 0, 0" "0.700000,0.700000,0.700000")))
    (Transformation|AttachComponentToComponent _returnvalue_5 _topview "None" "KeepRelative" "KeepRelative" "KeepRelative" true)
    (bind _returnvalue_6 (AddComponent|AddSplineMeshComponent false))
    (Transformation|AttachComponentToComponent _returnvalue_6 _topview_2 "None" "KeepRelative" "KeepRelative" "KeepRelative" true)
    (SplineMesh|SetStartandEnd _returnvalue_6 (.Location (Spline|GetLocationandTangentatSplinePoint _spline _index "Local")) (.Tangent (Spline|GetLocationandTangentatSplinePoint _spline _index "Local")) (.Location (Spline|GetLocationandTangentatSplinePoint _spline (+ _index 1) "Local")) (.Tangent (Spline|GetLocationandTangentatSplinePoint _spline (+ _index 1) "Local")) true :!class /Script/Engine.SplineMeshComponent)
    (Utilities|FlowControl|Delay 5.0)
    (Actor|DestroyActor)))

(event Collision|EventActorBeginOverlap
  (params (OtherActor :type Actor%20Object%20Reference)))

(event EventTick
  (params (DeltaSeconds :type Float%20%28single-precision%29)))

(fn ConstructionScript)