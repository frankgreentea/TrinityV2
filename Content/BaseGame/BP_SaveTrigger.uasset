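; Checkpoint trigger actor that, on overlap, writes its save number into its level's progress field in SaveSlot, then destroys itself.
; LevelsAVED selects the field, covering levels 3 through the final one, and a Reset event zeroes that field.
; Overlap also copies the player's temporary cutscene name into that level's entry unless it is "None".
; Hide and TwoSide control the meshes' visibility, with StaticMesh removed when not two-sided.
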(event Custom|Reset
  (bind _returnvalue (SaveGame|LoadGamefromSlot "SaveSlot"))
  (bind _asmy_save_game (Utilities|Casting|CastToMySaveGame _returnvalue))
  (switch int (Variables|Default|GetLevelsAVED)
    (:3
      (Variables|/Game/BaseGame/MySaveGame.MySaveGame_C|SetLevel3Progress _asmy_save_game 0))
    (:4
      (Variables|/Game/BaseGame/MySaveGame.MySaveGame_C|SetLevel4Progress _asmy_save_game 0))
    (:5
      (Variables|/Game/BaseGame/MySaveGame.MySaveGame_C|SetLevel5Progresss _asmy_save_game 0))
    (:6
      (Variables|/Game/BaseGame/MySaveGame.MySaveGame_C|SetLevel6Progress _asmy_save_game 0))
    (:7
      (Variables|/Game/BaseGame/MySaveGame.MySaveGame_C|SetLevel7Progress _asmy_save_game 0))
    (:8
      (Variables|/Game/BaseGame/MySaveGame.MySaveGame_C|SetLevel8Progress _asmy_save_game 0))
    (:9
      (Variables|/Game/BaseGame/MySaveGame.MySaveGame_C|SetLevel9Progress _asmy_save_game 0))
    (:10
      (Variables|/Game/BaseGame/MySaveGame.MySaveGame_C|SetLevelFinalProgress _asmy_save_game 0)))
  (SaveGame|SaveGametoSlot _asmy_save_game "SaveSlot"))

(event EventBeginPlay
  (if (not (Variables|Default|GetTwoSide))
    (Components|DestroyComponent (Variables|Default|GetStaticMesh))))

(event EventTick
  (params (DeltaSeconds :type Float%20%28single-precision%29)))

(event Collision|EventActorBeginOverlap
  (params (OtherActor :type Actor%20Object%20Reference))
  (bind _levelsaved (Variables|Default|GetLevelsAVED))
  (bind _saveniumber (Variables|Default|GetSaveNiumber))
  (bind _asmy_character (Utilities|Casting|CastToMyCharacter (Game|GetPlayerCharacter 0)))
  (Development|PrintString (Utilities|GetDisplayName (Variables|Default|GetDefaultSceneRoot)))
  (bind _returnvalue (SaveGame|LoadGamefromSlot "SaveSlot"))
  (bind _asmy_save_game (Utilities|Casting|CastToMySaveGame _returnvalue))
  (if (Utilities|Name|Equal(Name) (Utilities|Array|Get(acopy) (Variables|/Game/BaseGame/MySaveGame.MySaveGame_C|GetCutSceneName _asmy_save_game) _levelsaved) "None")
    _
    (elif (Utilities|Name|Equal(Name) (Utilities|Array|Get(acopy) (Variables|/Game/BaseGame/MySaveGame.MySaveGame_C|GetCutSceneName _asmy_save_game) _levelsaved) "none")
      _
      (elif (Utilities|Name|Equal(Name) (Utilities|Array|Get(acopy) (Variables|/Game/BaseGame/MySaveGame.MySaveGame_C|GetCutSceneName _asmy_save_game) _levelsaved) "")
        _
        (else
          (Utilities|Array|SetArrayElem (Variables|/Game/BaseGame/MySaveGame.MySaveGame_C|GetCutSceneName _asmy_save_game) _levelsaved (Variables|/Game/BaseGame/MyCharacter.MyCharacter_C|GetTempoCutSceneName _asmy_character))))))
  (switch int _levelsaved
    (:3
      (Variables|/Game/BaseGame/MySaveGame.MySaveGame_C|SetLevel3Progress _asmy_save_game _saveniumber))
    (:4
      (Variables|/Game/BaseGame/MySaveGame.MySaveGame_C|SetLevel4Progress _asmy_save_game _saveniumber))
    (:5
      (Variables|/Game/BaseGame/MySaveGame.MySaveGame_C|SetLevel5Progresss _asmy_save_game _saveniumber))
    (:6
      (Variables|/Game/BaseGame/MySaveGame.MySaveGame_C|SetLevel6Progress _asmy_save_game _saveniumber))
    (:7
      (Variables|/Game/BaseGame/MySaveGame.MySaveGame_C|SetLevel7Progress _asmy_save_game _saveniumber))
    (:8
      (Variables|/Game/BaseGame/MySaveGame.MySaveGame_C|SetLevel8Progress _asmy_save_game _saveniumber))
    (:9
      (Variables|/Game/BaseGame/MySaveGame.MySaveGame_C|SetLevel9Progress _asmy_save_game _saveniumber))
    (:10
      (Variables|/Game/BaseGame/MySaveGame.MySaveGame_C|SetLevelFinalProgress _asmy_save_game _saveniumber)))
  (SaveGame|SaveGametoSlot _asmy_save_game "SaveSlot")
  (Actor|DestroyActor))

(fn ConstructionScript
  (bind _staticmesh (Variables|Default|GetStaticMesh))
  (if (Variables|Default|GetHide)
    (Rendering|SetVisibility (Variables|Default|GetStaticMesh) false false)
    (elif (not (Variables|Default|GetTwoSide))
      (Collision|SetCollisionEnabled _staticmesh "NoCollision")
      (Rendering|SetVisibility _staticmesh false false))))